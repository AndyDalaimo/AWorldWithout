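; BP_InteractiveComputer is a world item computer that shows a UI interface when the player interacts with it.
; On BeginPlay it creates a WBP_ComputerInterface widget and passes it a reference to itself.
; On GCComputerInteract, if the widget is not already shown, it blends the view to the computer, initializes the interface, then adds it to the viewport after a delay matching the blend.
; A CloseComputerInterface call exists but is unconnected.
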(event `self.ReceiveBeginPlay`
  (bind _returnvalue (`|CreateWidget` "/Game/Widgets/WBP_ComputerInterface.WBP_ComputerInterface_C" (`GameplayStatics.GetPlayerController` 0)))
  (bind _output_get (set `self.ComputerWidgetRef` _returnvalue))
  (`/Game/Widgets/WBP_ComputerInterface.SetComputerRef` _output_get self))

(event `self.GC_ComputerInteract`
  (bind _computerwidgetref (`self.ComputerWidgetRef`))
  (if (not (`Widget.IsInViewport` _computerwidgetref))
    (`PlayerController.SetViewTargetWithBlend` (`GameplayStatics.GetPlayerController` 0) self 1.0 "VTBlend_Linear" 0.0 false)
    (`/Game/Widgets/WBP_ComputerInterface.InitComputerInterface` _computerwidgetref)
    (`KismetSystemLibrary.Delay` 1.0)
    (`UserWidget.AddToViewport` _computerwidgetref 0)))

(fn `UserConstructionScript`)