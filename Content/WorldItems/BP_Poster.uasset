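; BP_Poster is an interactable world item that shows a procedurally generated title on a WBP_BookCover widget.
; Its completed action calls the parent, then builds the title and pushes it to the widget cached from DialogueWidget at BeginPlay.
; The title joins an article, adjective and noun from a DataTable, generated only once.
; Adjective and noun streams are seeded from actor location, but the article pick is unseeded.
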(event `self.ReceiveBeginPlay`
  (bind _aswbp_book_cover (cast `/Game/Widgets/WBP_BookCover` (`WidgetComponent.GetUserWidgetObject` (`self.DialogueWidget`))))
  (set `self.BookCoverWidgetRef` _aswbp_book_cover))

(event `InteractableInterface.ActionToComplete`
  (`parent.ActionToComplete`)
  (`self.GenerateRandomTitle` (`self.DT_TitleGenerator`))
  (`/Game/Widgets/WBP_BookCover.SetBookTitle` (`self.BookCoverWidgetRef`) (`self.Title`)))

(fn `GenerateRandomTitle`
  (params (DataTable :type "DataTable Object Reference"))
  (bind (_returnvalue_x _returnvalue_y _returnvalue_z) (`KismetMathLibrary.BreakVector` (`self.K2_GetActorLocation`)))
  (bind (_returnvalue_x_2 _returnvalue_y_2) (`KismetMathLibrary.BreakVector` (`self.K2_GetActorLocation`)))
  (if (`self.GeneratedTitle`)
    (`KismetSystemLibrary.PrintString` (`self.Title`))
    (else
      (`|ExecutionSequence`
        (:`then_0`
          (set `self.GeneratedTitle` true)
          (`KismetMathLibrary.SetRandomStreamSeed` (`self.AdjectiveStream`) (`KismetMathLibrary.FTrunc` (+ _returnvalue_x _returnvalue_y _returnvalue_z)))
          (`KismetMathLibrary.SetRandomStreamSeed` (`self.NounStream`) (`KismetMathLibrary.FTrunc` (+ _returnvalue_x_2 _returnvalue_y_2 0.0)))
          (bind _returnvalue (`|GetDataTableRow` DataTable (`KismetStringLibrary.Conv_StringToName` (`KismetStringLibrary.Concat_StrStr` (`self.RowName`) (`KismetStringLibrary.Conv_IntToString` (`KismetMathLibrary.RandomIntegerInRange` 0 2)))))
            (:`then`
              (set `self.Title` (`KismetStringLibrary.Concat_StrStr` (`self.Title`) (`.Articles` (break `TitleGenerator` _returnvalue)) " ")))))
        (:`then_1`
          (bind _returnvalue_2 (`|GetDataTableRow` DataTable (`KismetStringLibrary.Conv_StringToName` (`KismetStringLibrary.Concat_StrStr` (`self.RowName`) (`KismetStringLibrary.Conv_IntToString` (`KismetMathLibrary.RandomIntegerInRangeFromStream` (`self.AdjectiveStream`) 0 227)))))
            (:`then`
              (set `self.Title` (`KismetStringLibrary.Concat_StrStr` (`self.Title`) (`.Adjectives` (break `TitleGenerator` _returnvalue_2)) " ")))
            (:`RowNotFound`
              (`KismetSystemLibrary.PrintString` "Not Working"))))
        (:`then_2`
          (bind _returnvalue_3 (`|GetDataTableRow` DataTable (`KismetStringLibrary.Conv_StringToName` (`KismetStringLibrary.Concat_StrStr` (`self.RowName`) (`KismetStringLibrary.Conv_IntToString` (`KismetMathLibrary.RandomIntegerInRangeFromStream` (`self.NounStream`) 0 384)))))
            (:`then`
              (bind _output_get (set `self.Title` (`KismetStringLibrary.Concat_StrStr` (`self.Title`) (`.Nouns` (break `TitleGenerator` _returnvalue_3)))))
              (`KismetSystemLibrary.PrintString` _output_get))))))))

(fn `UserConstructionScript`)