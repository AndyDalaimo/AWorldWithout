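; BP_BaseInteractableActor is a base Blueprint for interactable world actors that display dialogue through a widget component.
; On BeginPlay it caches the DialogueWidget's user widget as a WBP_Dialogue reference.
; ActiontoComplete runs the parent behavior, then pushes the current dialogue from InteractComp's InteractData into that widget.
; It sets the title only while the data's bSpokenTo flag is false.
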(event `self.ReceiveBeginPlay`
  (bind _aswbp_dialogue (cast `/Game/Widgets/WBP_Dialogue` (`WidgetComponent.GetUserWidgetObject` (`self.DialogueWidget`))))
  (set `self.DialogueWidgetRef` _aswbp_dialogue))

(event `InteractableInterface.ActionToComplete`
  (bind (_interactdata_interactabletype _interactdata_bspokento _interactdata_title _interactdata_currentdialogue) (break `InteractData` (`AC_Interactable.InteractData` (`self.InteractComp`))))
  (`parent.ActionToComplete`)
  (`/Game/Widgets/WBP_Dialogue.SetCurrentDialogue` (`self.DialogueWidgetRef`) _interactdata_currentdialogue)
  (if (not _interactdata_bspokento)
    (`/Game/Widgets/WBP_Dialogue.SetTitle` (`self.DialogueWidgetRef`) _interactdata_title)))

(fn `UserConstructionScript`)